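; Hub manager that handles dice results to open portals or move the player across hub fields, registering itself with BP_GameModeMain.
; HandleDiceResult closes three portals, then opens the one matching a roll of 1–3.
; StartMoveByDice recursively follows NextField links, issuing SimpleMoveToLocation at each step without waiting for arrival, then resolves the final field's theme.
; DisableAllPortals and OpenPortalByTheme are empty; the theme-to-portal switch is unconnected.
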(event EventBeginPlay
  (bind _asbp_game_mode_main (Utilities|Casting|CastToBP_GameModeMain (Game|GetGameMode)))
  (Default|RegisterManagers _asbp_game_mode_main 0 self))

(event Collision|EventActorBeginOverlap
  (params (OtherActor :type Actor%20Object%20Reference)))

(event EventTick
  (params (DeltaSeconds :type Float%20%28single-precision%29)))

(fn ConstructionScript)

(fn HandleDiceResult
  (params (DiceValue :type Integer))
  (bind _output_get (Variables|Default|SetLastDiceValue DiceValue))
  (Development|PrintString (Utilities|String|Append "Dice Value : " (Utilities|String|ToString(Integer) _output_get)))
  (Default|ClosePortal (Variables|Default|GetPortalARef))
  (Default|ClosePortal (Variables|Default|GetPortalBRef))
  (Default|ClosePortal (Variables|Default|GetPortalCRef))
  (switch int (Variables|Default|GetLastDiceValue)
    (:1
      (Default|OpenPortal (Variables|Default|GetPortalARef)))
    (:2
      (Default|OpenPortal (Variables|Default|GetPortalBRef)))
    (:3
      (Default|OpenPortal (Variables|Default|GetPortalCRef)))))

(fn StartMovebyDice
  (params (DiceValue :type Integer))
  (Variables|Default|SetRemainingMoveCount DiceValue)
  (Variables|Default|SetIsMovingOnHub true)
  (CallFunction|DisableAllPortals)
  (CallFunction|MoveNextField))

(fn DisableAllPortals)

(fn MoveNextField
  (if (<= (Variables|Default|GetRemainingMoveCount) 0)
    (Variables|Default|SetIsMovingOnHub false)
    (CallFunction|ResolveCurrentFieldTheme)
    (else
      (bind _output_get (Variables|Default|SetTargetFieldRef (Variables|/Game/Blueprints/Hub/BP_HubFieldBase.BP_HubFieldBase_C|GetNextField (Variables|Default|GetCurrentFieldRef))))
      (bind _output_get_2 (Variables|Default|SetCurrentFieldRef _output_get))
      (CallFunction|MovePlayertoField _output_get_2)
      (bind _result (Math|Integer|DecrementInt (Variables|Default|GetRemainingMoveCount))
        (:%20%20
          (Variables|Default|SetRemainingMoveCount _result)
          (CallFunction|MoveNextField))))))

(fn MovePlayertoField
  (params (InFieldRef :type BP%20Hub%20Field%20Base%20Object%20Reference))
  (AI|Navigation|SimpleMovetoLocation (Pawn|GetController (Variables|Default|GetPlayerRef)) (Transformation|GetActorLocation InFieldRef)))

(fn ResolveCurrentFieldTheme
  (CallFunction|OpenPortalbyTheme (Variables|/Game/Blueprints/Hub/BP_HubFieldBase.BP_HubFieldBase_C|GetThemeType (Variables|Default|GetCurrentFieldRef))))

(fn OpenPortalbyTheme
  (params (InThemeType :type E_ThemeType%20Enum :default "NewEnumerator0")))