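; BP_ThemePortalBase is a base theme portal actor that opens and closes on demand.
; OpenPortal finds BP_HubManager, teleports the portal to the X/Y of the manager's current field at a fixed height, then shows it and enables query-only box collision.
; ClosePortal hides the Portal component and disables the box collision.
; The overlap event is empty, so this Blueprint defines no behavior on entering the portal.
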(event EventBeginPlay)

(event Collision|EventActorBeginOverlap
  (params (OtherActor :type Actor%20Object%20Reference)))

(event EventTick
  (params (DeltaSeconds :type Float%20%28single-precision%29)))

(fn ConstructionScript)

(fn OpenPortal
  (bind _returnvalue (Actor|GetActorOfClass "/Game/Blueprints/Hub/BP_HubManager.BP_HubManager_C"))
  (Transformation|SetActorLocation (Math|Vector|MakeVector (.x (Transformation|GetActorLocation (Variables|/Game/Blueprints/Hub/BP_HubManager.BP_HubManager_C|GetCurrentFieldRef _returnvalue))) (.y (Transformation|GetActorLocation (Variables|/Game/Blueprints/Hub/BP_HubManager.BP_HubManager_C|GetCurrentFieldRef _returnvalue))) 2.6e+02) false true)
  (Rendering|SetVisibility (Variables|Default|GetPortal) true true)
  (Collision|SetCollisionEnabled (Variables|Default|GetBoxCollision) "QueryOnly"))

(fn ClosePortal
  (Rendering|SetVisibility (Variables|Default|GetPortal) false false)
  (Collision|SetCollisionEnabled (Variables|Default|GetBoxCollision) "NoCollision"))