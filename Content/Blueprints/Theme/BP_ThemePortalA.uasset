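; BP_ThemePortalA is a portal that moves the player to a fixed spot near the world origin on overlap.
; It first saves an offset return location and the player's rotation in BP_GameMode, and starts a level sequence.
; After the move it sets game-only input, hides the cursor and stops character movement.
; SetPortalEnabled stores CanEnter and opens or closes the portal, but the overlap never checks that flag.
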(event Collision|EventActorBeginOverlap
  (params (OtherActor :type Actor%20Object%20Reference))
  (bind _returnvalue (Game|GetPlayerController 0))
  (if (Actor|ActorHasTag OtherActor "Player")
    (bind _asbp_game_mode (Utilities|Casting|CastToBP_GameMode (Game|GetGameMode)))
    (Variables|/Game/Blueprints/Character/BP_GameMode.BP_GameMode_C|SetReturnLocation _asbp_game_mode (+ (Transformation|GetActorLocation OtherActor) "150.000000,150.000000,0.000000"))
    (Variables|/Game/Blueprints/Character/BP_GameMode.BP_GameMode_C|SetReturnRotation _asbp_game_mode (Transformation|GetActorRotation OtherActor))
    (bind _returnvalue_2 (Sequencer|Player|CreateLevelSequencePlayer "/Game/Blueprints/LevelSequence/PortalLevelSequence.PortalLevelSequence"))
    (Sequencer|Player|Play _returnvalue_2 :!class /Script/MovieScene.MovieSceneSequencePlayer)
    (Transformation|SetActorLocation OtherActor "0.000000,0.000000,88.000000" false false)
    (Input|SetInputModeGameOnly _returnvalue false)
    (Variables|/Script/Engine.PlayerController|SetbShowMouseCursor _returnvalue false)
    (bind _ascharacter (Utilities|Casting|CastToCharacter OtherActor))
    (Components|Movement|StopMovementImmediately (Variables|/Script/Engine.Character|GetCharacterMovement _ascharacter))))

(fn ConstructionScript
  (|CallParentFunction))

(fn SetPortalEnabled
  (params (InCanEnter :type Boolean))
  (bind _output_get (Variables|Default|SetCanEnter InCanEnter))
  (if _output_get
    (CallFunction|OpenPortal)
    (else
      (CallFunction|ClosePortal))))