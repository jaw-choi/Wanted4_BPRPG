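; BP_Dice is a physics die that can be rolled, read, hidden and placed on the current field.
; Roll launches the Cube upward with random force and spins it with random torque around a random axis.
; GetTopFaceVal maps the dominant world-axis component of the Cube's up vector to a value from one to six, printing it.
; AppearInFrontOfPlayer teleports the die to BP_HubManager's CurrentFieldRef and shows it, while Disappear hides it.
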(event EventBeginPlay)

(event Collision|EventActorBeginOverlap
  (params (OtherActor :type Actor%20Object%20Reference)))

(event EventTick
  (params (DeltaSeconds :type Float%20%28single-precision%29)))

(fn ConstructionScript)

(fn Roll
  (Physics|AddForce (Variables|Default|GetCube) (* (Math|Random|RandomFloatinRange 4e+04 5e+04) "0.000000,0.000000,1.000000") "None" true)
  (Class|PrimitiveComponent|AddTorqueinDegrees (Variables|Default|GetCube) (* (Math|Random|RandomFloatinRange 2.5e+04 3e+04) (Math|Random|RandomUnitVector)) "None" true))

(fn GetTopFaceVal
  (if (<= (.Y (Math|Vector|BreakVector (Math|Vector|GetUpVector (Variables|Default|GetCube)))) -0.9)
    (Development|PrintString "1")
    (return 1)
    (elif (>= (.Y (Math|Vector|BreakVector (Math|Vector|GetUpVector (Variables|Default|GetCube)))) 0.9)
      (Development|PrintString "6")
      (return 6)
      (elif (>= (.Z (Math|Vector|BreakVector (Math|Vector|GetUpVector (Variables|Default|GetCube)))) 0.9)
        (Development|PrintString "3")
        (return 3)
        (elif (<= (.Z (Math|Vector|BreakVector (Math|Vector|GetUpVector (Variables|Default|GetCube)))) -0.9)
          (Development|PrintString "4")
          (return 4)
          (elif (<= (.X (Math|Vector|BreakVector (Math|Vector|GetUpVector (Variables|Default|GetCube)))) -0.9)
            (Development|PrintString "5")
            (return 5)
            (elif (>= (.X (Math|Vector|BreakVector (Math|Vector|GetUpVector (Variables|Default|GetCube)))) 0.9)
              (Development|PrintString "2")
              (return 2))))))))

(fn Disappear
  (Rendering|SetVisibility (Variables|Default|GetCube) false false))

(fn AppearinFrontOfPlayer
  (bind _returnvalue (Actor|GetActorOfClass "/Game/Blueprints/Hub/BP_HubManager.BP_HubManager_C"))
  (Transformation|SetActorLocation (Transformation|GetActorLocation (Variables|/Game/Blueprints/Hub/BP_HubManager.BP_HubManager_C|GetCurrentFieldRef _returnvalue)) false true)
  (Rendering|SetVisibility (Variables|Default|GetCube) true false))