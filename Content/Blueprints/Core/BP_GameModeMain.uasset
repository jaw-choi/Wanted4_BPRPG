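; Main game mode that tracks turns, per-theme visit counts, skill flags and boss unlock.
; Theme visits escalate rewards: stat boost, skill grant, then a one-time upgrade.
; CheckBossUnlock sets a flag once the turn threshold is reached, but nothing here calls it.
; Stat rewards only print, RequestHubRefresh is empty, and RegisterManagers stores only the hub manager because the dice manager branch is disconnected.
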(fn ConstructionScript)

(fn RegisterManagers
  (params (InDiceManager :type BP%20Dice%20Manager%20Object%20Reference) (InHubManager :type BP%20Hub%20Manager%20Object%20Reference))
  (Utilities|IsValid InHubManager
    (:Is%20Valid
      (Variables|Default|SetHubManagerRef InHubManager))))

(fn AdvanceTurn
  (bind _result (Math|Integer|IncrementInt (Variables|Default|GetCurrentTurn))
    (:%20%20
      (bind _output_get (Variables|Default|SetCurrentTurn _result))
      (Development|PrintString (Utilities|String|Append "Current Turn : " (Utilities|String|ToString(Integer) _output_get))))))

(fn ProcessThemeVisit
  (params (ThemeType :type E_ThemeType%20Enum :default "NewEnumerator0"))
  (switch Utilities|FlowControl|Switch|SwitchonE_ThemeType ThemeType
    (:NewEnumerator1
      (bind _result (Math|Integer|IncrementInt (Variables|Default|GetVisitCountA))
        (:%20%20
          (bind _output_get (Variables|Default|SetVisitCountA _result))
          (CallFunction|ApplyThemeReward "NewEnumerator1" _output_get))))
    (:NewEnumerator2
      (bind _result_2 (Math|Integer|IncrementInt (Variables|Default|GetVisitCountB))
        (:%20%20
          (bind _output_get_2 (Variables|Default|SetVisitCountB _result_2))
          (CallFunction|ApplyThemeReward "NewEnumerator2" _output_get_2))))
    (:NewEnumerator3
      (bind _result_3 (Math|Integer|IncrementInt (Variables|Default|GetVisitCountC))
        (:%20%20
          (bind _output_get_3 (Variables|Default|SetVisitCountC _result_3))
          (CallFunction|ApplyThemeReward "NewEnumerator3" _output_get_3))))))

(fn ApplyThemeReward
  (params (ThemeType :type E_ThemeType%20Enum :default "NewEnumerator0") (VisitCount :type Integer))
  (switch int VisitCount
    (:1
      (CallFunction|ApplyStatReward ThemeType))
    (:2
      (CallFunction|GrantThemeSkill ThemeType))
    (:3
      (CallFunction|UpgradeThemeSkill ThemeType :!label _label))
    (:4
      (goto _label))))

(fn CheckBossUnlock
  (if (>= (Variables|Default|GetCurrentTurn) (Variables|Default|GetBossOpenTurn))
    (if (not (Variables|Default|GetBossUnlocked))
      (Variables|Default|SetBossUnlocked true)
      (Development|PrintString "Boss Unlocked"))))

(fn RequestHubRefresh)

(fn ApplyStatReward
  (params (ThemeType :type E_ThemeType%20Enum :default "NewEnumerator0"))
  (switch Utilities|FlowControl|Switch|SwitchonE_ThemeType ThemeType
    (:NewEnumerator1
      (Development|PrintString "A stat up"))
    (:NewEnumerator2
      (Development|PrintString "B stat up"))
    (:NewEnumerator3
      (Development|PrintString "C stat up"))))

(fn GrantThemeSkill
  (params (ThemeType :type E_ThemeType%20Enum :default "NewEnumerator0"))
  (switch Utilities|FlowControl|Switch|SwitchonE_ThemeType ThemeType
    (:NewEnumerator1
      (Variables|Default|SetHasSkillA true)
      (Development|PrintString "A skill granted"))
    (:NewEnumerator2
      (Variables|Default|SetHasSkillB true)
      (Development|PrintString "B skill granted"))
    (:NewEnumerator3
      (Variables|Default|SetHasSkillC true)
      (Development|PrintString "C skill granted"))))

(fn UpgradeThemeSkill
  (params (ThemeType :type E_ThemeType%20Enum :default "NewEnumerator0"))
  (switch Utilities|FlowControl|Switch|SwitchonE_ThemeType ThemeType
    (:NewEnumerator1
      (if (not (Variables|Default|GetSkillUpgradedA))
        (Variables|Default|SetSkillUpgradedA true)
        (Development|PrintString "A skill upgraded")))
    (:NewEnumerator2
      (if (not (Variables|Default|GetSkillUpgradedB))
        (Variables|Default|SetSkillUpgradedB true)
        (Development|PrintString "B skill upgraded")))
    (:NewEnumerator3
      (if (not (Variables|Default|GetSkillUpgradedC))
        (Variables|Default|SetSkillUpgradedC true)
        (Development|PrintString "C skill upgraded")))))